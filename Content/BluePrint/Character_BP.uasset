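; Player character for a touch-controlled RPG, driven by a virtual joystick or input axes, with movement blocked while attacking.
; BeginPlay spawns the inventory actor, loads saved stats and items, derives combat stats from attributes, and lays out skill and potion buttons.
; Skills 1-2 play attack montages, Skill 3 grants items, and Skill 4 quits after repeated taps.
; Touches reach the UTC input manager only while UI is closed; Back saves and exits.
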(event OnTap(Skill_1)
  (params (Location :type Vector :default "0, 0, 0") (FingerIndex :type ETouchIndex%20Enum :default "Touch1"))
  ;[1 0 0.8618] Skill
  (if (not (Variables|Default|GetisAttack))
    (Variables|Default|SetisAttack true)
    (Animation|Montage|MontagePlay (Components|SkeletalMesh|GetAnimInstance (Variables|Character|GetMesh)) "/Game/Character/animation/AttackAnimMontage.AttackAnimMontage" (Variables|Default|GetAttackSpeed) "MontageLength" 0.0)))

(event OnTap(Skill_2)
  (params (Location :type Vector :default "0, 0, 0") (FingerIndex :type ETouchIndex%20Enum :default "Touch1"))
  ;[1 0 0.8618] Skill
  (if (not (Variables|Default|GetisAttack))
    (Variables|Default|SetisAttack true)
    (Animation|Montage|MontagePlay (Components|SkeletalMesh|GetAnimInstance (Variables|Character|GetMesh)) "/Game/Character/animation/MagicAttackAnimMontage.MagicAttackAnimMontage" (Variables|Default|GetAttackSpeed) "MontageLength" 0.0)))

(event OnXAxisChanged(MovementJoystick)
  (params (Value :type Float%20%28single-precision%29))
  ;[0 1 0] Movement
  (if (not (Variables|Default|GetisAttack))
    (Pawn|Input|AddMovementInput "1.000000,0.000000,0.000000" (* Value (Variables|/Script/Amody.UserData|GetmoveSpeed (Variables|Default|GetUserData))) false)))

(event OnYAxisChanged(MovementJoystick)
  (params (Value :type Float%20%28single-precision%29))
  ;[0 1 0] Movement
  (if (not (Variables|Default|GetisAttack))
    (Pawn|Input|AddMovementInput "0.000000,-1.000000,0.000000" (* (Variables|/Script/Amody.UserData|GetmoveSpeed (Variables|Default|GetUserData)) Value) false)))

(event OnTap(Skill_3)
  (params (Location :type Vector :default "0, 0, 0") (FingerIndex :type ETouchIndex%20Enum :default "Touch1"))
  (bind _inventoryref (Variables|Default|GetInventoryRef))
  ;[1 0 0.8618] Skill
  (Default|AddItem _inventoryref "/Game/Item/ItmeRing_BP.ItmeRing_BP_C" 1)
  (Default|AddItem _inventoryref "/Game/Item/HealthPotionItem_BP.HealthPotionItem_BP_C" 30)
  (Development|PrintString "Ring 1개 획득!!")
  (Development|PrintString "Health Potion 30개 획득!!"))

(event OnTap(Skill_4)
  (params (Location :type Vector :default "0, 0, 0") (FingerIndex :type ETouchIndex%20Enum :default "Touch1"))
  ;[1 0 0.8618] Skill
  ;[1 1 1] Exit Game
  (switch int (Variables|Default|GetExitTouchCount)
    (:Default
      (Development|ExecuteConsoleCommand "exit" :!label _label))
    (:0
      (Math|Integer|IncrementInt (Variables|Default|GetExitTouchCount)
        (:%20%20
          (Development|PrintString "종료 하시겠습니까?")
          (Utilities|FlowControl|Delay 3.0)
          (Variables|Default|SetExitTouchCount 0))))
    (:1
      (Math|Integer|IncrementInt (Variables|Default|GetExitTouchCount)
        (:%20%20
          (Development|PrintString "진짜 종료 하시겠습니까?"))))
    (:2
      (Math|Integer|IncrementInt (Variables|Default|GetExitTouchCount)
        (:%20%20
          (Development|PrintString "진짜 진짜 종료 하시겠습니까?"))))
    (:3
      (goto _label))))

(event Collision|EventActorBeginOverlap
  (params (OtherActor :type Actor%20Object%20Reference)))

(event EventBeginPlay
  (bind _movementjoystick (Variables|Default|GetMovementJoystick))
  ;[1 1 1] Inventory Actor Spawn
  (bind _returnvalue (Game|SpawnActorfromClass "/Game/UI/Inventory/BP/Inventory_BP.Inventory_BP_C" (Math|Transform|MakeTransform "0, 0, 0" "0, 0, 0" "1,1,1") "Undefined" 0 100 self 0 5 0))
  (bind _output_get (Variables|Default|SetInventoryRef _returnvalue))
  (Variables|Default|SetPlayerUI (Variables|/Game/UI/Inventory/BP/Inventory_BP.Inventory_BP_C|GetPlayerUI _output_get))
  ;[0 0.5358 1] CheckBounds
  (Default|SetupBounds _movementjoystick true "(X=0.000000,Y=0.600000)" "(X=0.300000,Y=0.400000)" true false)
  (Variables|/Game/JoystickCore/UTCComponent.UTCComponent_C|SetPriority _movementjoystick 1)
  (Default|SetupWidget (Variables|Default|GetMovementJoystick) "/Game/JoystickCore/Widgets/AnimatedWidgets/JoystickWidgetAnimated.JoystickWidgetAnimated_C" true true)
  ;[0.1006 1 0] Setup
  (CallFunction|LoadData)
  (CallFunction|SetupData)
  (CallFunction|MakeUserData)
  (CallFunction|SetupSkill)
  (Default|UpdateEquipmentSlot (Variables|/Game/UI/PlayerUI.PlayerUI_C|GetEquipment_widget (Variables|Default|GetPlayerUI))))

(event EventTick
  (params (DeltaSeconds :type Float%20%28single-precision%29)))

(event Input|ActionEvents|InputActionBackButton
  (params (Key :type Key%20Structure))
  ;[1 1 1] Exit Game
  (:Pressed
    (bind _foundwidgets (Widget|GetAllWidgetsOfClass "/Game/UI/PlayerUI.PlayerUI_C" true))
    (Default|SaveGame (Utilities|Array|Get(acopy) _foundwidgets))
    (Development|ExecuteConsoleCommand "exit")
    (switch int (Variables|Default|GetExitTouchCount)
      (:Default
        (Development|ExecuteConsoleCommand "exit" :!label _label))
      (:0
        (Math|Integer|IncrementInt (Variables|Default|GetExitTouchCount)
          (:%20%20
            (Development|PrintString "종료 하시겠습니까?")
            (Utilities|FlowControl|Delay 3.0)
            (Variables|Default|SetExitTouchCount 0))))
      (:1
        (Math|Integer|IncrementInt (Variables|Default|GetExitTouchCount)
          (:%20%20
            (Development|PrintString "진짜 종료 하시겠습니까?"))))
      (:2
        (Math|Integer|IncrementInt (Variables|Default|GetExitTouchCount)
          (:%20%20
            (Development|PrintString "진짜 진짜 종료 하시겠습니까?"))))
      (:3
        (goto _label)))))

(event Input|AxisEvents|InputAxisAxisX
  (params (AxisValue :type Float%20%28single-precision%29))
  ;[0 0 0] Keybord Movemet
  (if (not (Variables|Default|GetisAttack))
    (Pawn|Input|AddMovementInput "1.000000,0.000000,0.000000" (* AxisValue (Variables|/Script/Amody.UserData|GetmoveSpeed (Variables|Default|GetUserData))) false)))

(event Input|AxisEvents|InputAxisAxisY
  (params (AxisValue :type Float%20%28single-precision%29))
  ;[0 0 0] Keybord Movemet
  (if (not (Variables|Default|GetisAttack))
    (Pawn|Input|AddMovementInput "0.000000,-1.000000,0.000000" (* (Variables|/Script/Amody.UserData|GetmoveSpeed (Variables|Default|GetUserData)) AxisValue) false)))

(event Input|TouchEvents|InputTouch
  (params (Location :type Vector) (FingerIndex :type ETouchIndex%20Enum))
  ;[0.1006 1 0] Setup
  (:Pressed
    (if (not (Variables|Default|GetisUiOpen))
      (Utilities|UTCTouchInputManager Location FingerIndex :!label _label)))
  (:Released
    (goto _label Released))
  (:Moved
    (goto _label Moved)))

(fn ConstructionScript)

(fn LoadData
  (bind _inventoryref (Variables|Default|GetInventoryRef))
  (bind _returnvalue (SaveGame|DoesSaveGameExist (Variables|Default|GetSaveGameSlotName)))
  (if _returnvalue
    (bind _returnvalue_2 (SaveGame|LoadGamefromSlot (Variables|Default|GetSaveGameSlotName)))
    (Variables|Default|SetSaverSubClass _returnvalue_2)
    (bind _assave_object_bp (Utilities|Casting|CastToSaveObject_BP (Variables|Default|GetSaverSubClass))
      (:then
        (Variables|Save|SetSaveUserData (Variables|/Game/BluePrint/SaveObject_BP.SaveObject_BP_C|GetUserData _assave_object_bp))
        (bind _output_get (Variables|/Game/UI/Inventory/BP/Inventory_BP.Inventory_BP_C|Setslot _inventoryref (Variables|/Game/BluePrint/SaveObject_BP.SaveObject_BP_C|GetInventoryData _assave_object_bp)))
        (for (_ _array_index) _output_get
          (Default|UpdateSlotatIndex _inventoryref _array_index)))
      (:CastFailed
        (Development|PrintString "Error! - Casting Fail")))
    (else
      (bind _returnvalue_3 (SaveGame|CreateSaveGameObject "/Game/BluePrint/SaveObject_BP.SaveObject_BP_C"))
      (Variables|Default|SetSaverSubClass _returnvalue_3)
      (bind _assave_object_bp_2 (Utilities|Casting|CastToSaveObject_BP (Variables|Default|GetSaverSubClass))
        (:then
          (Variables|/Game/BluePrint/SaveObject_BP.SaveObject_BP_C|SetUserData _assave_object_bp_2 (Variables|Save|GetSaveUserData)))
        (:CastFailed
          (Development|PrintString "Error! - Casting Fail"))))))

(fn SetupData
  (bind _saveuserdata (Variables|Save|GetSaveUserData))
  (bind _userdata (Variables|Default|GetUserData))
  (bind (_level _exp _strength _agility _intelligence _vitality _energy _hp _mp _statspoint) (Utilities|Struct|BreakSavedUserDataStruct _saveuserdata))
  (Variables|/Script/Amody.UserData|Setlevel _userdata _level)
  (Variables|/Script/Amody.UserData|Setexp _userdata _exp)
  (Variables|/Script/Amody.UserData|Setstrength _userdata _strength)
  (Variables|/Script/Amody.UserData|Setagility _userdata _agility)
  (Variables|/Script/Amody.UserData|Setintelligence _userdata _intelligence)
  (Variables|/Script/Amody.UserData|Setvitality _userdata _vitality)
  (Variables|/Script/Amody.UserData|Setenergy _userdata _energy)
  (Variables|/Script/Amody.UserData|Sethp _userdata _hp)
  (Variables|/Script/Amody.UserData|Setmp _userdata _mp)
  (Variables|/Script/Amody.UserData|SetstatsPoint _userdata _statspoint))

(fn MakeUserData
  (bind _userdata (Variables|Default|GetUserData))
  (bind _userdata_2 (Variables|Default|GetUserData))
  (bind _userdata_3 (Variables|Default|GetUserData))
  (bind _userdata_4 (Variables|Default|GetUserData))
  (bind _userdata_5 (Variables|Default|GetUserData))
  (bind _userdata_6 (Variables|Default|GetUserData))
  (bind _userdata_7 (Variables|Default|GetUserData))
  (bind _userdata_8 (Variables|Default|GetUserData))
  (bind _userdata_9 (Variables|Default|GetUserData))
  (bind _userdata_10 (Variables|Default|GetUserData))
  (bind _userdata_11 (Variables|Default|GetUserData))
  (bind _strength (Variables|/Script/Amody.UserData|Getstrength _userdata))
  (bind _damageperstrength (Variables|/Script/Amody.UserData|GetDamagePerStrength _userdata))
  (bind _vitality (Variables|/Script/Amody.UserData|Getvitality _userdata_3))
  (bind _agility (Variables|/Script/Amody.UserData|Getagility _userdata_2))
  (bind _returnvalue (* _strength _damageperstrength))
  (Variables|/Script/Amody.UserData|SetminAttackDamage _userdata_8 (Math|Float|Truncate _returnvalue))
  (Variables|/Script/Amody.UserData|SetmaxAttackDamage _userdata_8 (Math|Float|Truncate (* _returnvalue 2.0)))
  (Variables|/Script/Amody.UserData|SethpMax _userdata_9 (Math|Float|Truncate (* _vitality (Variables|/Script/Amody.UserData|GethpPerVitality _userdata_3))))
  (Variables|/Script/Amody.UserData|SethpRecoveryForSecond _userdata_9 (* _vitality (Variables|/Script/Amody.UserData|GethpRecoverPerVitality _userdata_3)))
  (Variables|/Script/Amody.UserData|SetmoveSpeed _userdata_4 (Variables|Default|GetMoveSpeed))
  (Variables|/Script/Amody.UserData|SetattackSpeed _userdata_4 (Variables|Default|GetAttackSpeed))
  (Variables|/Script/Amody.UserData|SetmagicDamage _userdata_5 (Math|Float|Truncate (* (Variables|/Script/Amody.UserData|Getintelligence _userdata_6) (Variables|/Script/Amody.UserData|GetmagicDamagePerIntelligence _userdata_6))))
  (Variables|/Script/Amody.UserData|SetattackRate _userdata_5 (Math|Float|Truncate (* _agility (Variables|/Script/Amody.UserData|GetattackRatePerAgility _userdata_6))))
  (Variables|/Script/Amody.UserData|Setdefense _userdata_7 (Math|Float|Truncate (* _agility (Variables|/Script/Amody.UserData|GetdefencePerAgility _userdata_2))))
  (Variables|/Script/Amody.UserData|SetblockRate _userdata_7 (Variables|Default|GetBolokRate))
  (Variables|/Script/Amody.UserData|SetfireAttack _userdata_10 (Variables|Default|GetFireAttack))
  (Variables|/Script/Amody.UserData|SeticeAttack _userdata_10 (Variables|Default|GetIceAttack))
  (Variables|/Script/Amody.UserData|SetlightningAttack _userdata_10 (Variables|Default|GetLightningAttack))
  (Variables|/Script/Amody.UserData|SetpoisonAttack _userdata_10 (Variables|Default|GetPoisonAttack))
  (Variables|/Script/Amody.UserData|SethpAbsorb _userdata_11 (Variables|Default|GetHpAbsorb))
  (Variables|/Script/Amody.UserData|SetmpAbsorb _userdata_11 (Variables|Default|GetMpAbsorb))
  (Variables|/Script/Amody.UserData|SetmagicChance (Variables|Default|GetUserData) (Variables|Default|GetMagicChance)))

(fn SetupSkill
  (bind _skill_4 (Variables|Default|GetSkill_4))
  (bind _potion1 (Variables|Default|GetPotion1))
  (bind _potion2 (Variables|Default|GetPotion2))
  (bind _skill_3 (Variables|Default|GetSkill_3))
  (bind _skill_2 (Variables|Default|GetSkill_2))
  (bind _skill_1 (Variables|Default|GetSkill_1))
  (Utilities|FlowControl|Sequence
    (:then_0
      (Default|SetupBounds _skill_1 true "(X=0.900000,Y=0.800000)" "(X=0.000000,Y=0.150000)" true true)
      (Default|SetupBackgroundbyBounds _skill_1 "/Game/Skill_Icon/Skill_1_Widget.Skill_1_Widget_C" true)
      (Default|SetupBounds _skill_2 true "(X=0.900000,Y=0.600000)" "(X=0.000000,Y=0.150000)" true true)
      (Default|SetupBackgroundbyBounds _skill_2 "/Game/Skill_Icon/Skill_2_Widget.Skill_2_Widget_C" true))
    (:then_1
      (Default|SetupBounds _skill_3 true "(X=0.900000,Y=0.400000)" "(X=0.000000,Y=0.150000)" true true)
      (Default|SetupBackgroundbyBounds _skill_3 "/Game/Skill_Icon/Skill_3_Widget.Skill_3_Widget_C" true)
      (Default|SetupBounds _skill_4 true "(X=0.900000,Y=0.200000)" "(X=0.000000,Y=0.150000)" true true)
      (Default|SetupBackgroundbyBounds _skill_4 "/Game/Skill_Icon/Skill_4_Widget.Skill_4_Widget_C" true))
    (:then_2
      (Default|SetupBounds _potion1 true "(X=0.700000,Y=0.800000)" "(X=0.000000,Y=0.150000)" true true)
      (Default|SetupBackgroundbyBounds _potion1 "/Game/JoystickCore/Widgets/AnimatedWidgets/Potion_1_Widget.Potion_1_Widget_C" true)
      (Default|SetupBounds _potion2 true "(X=0.800000,Y=0.800000)" "(X=0.000000,Y=0.150000)" true true)
      (Default|SetupBackgroundbyBounds _potion2 "/Game/JoystickCore/Widgets/AnimatedWidgets/Potion_2_Widget.Potion_2_Widget_C" true))))