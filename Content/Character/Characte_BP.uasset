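; Player character for a touch-screen game, with movement, a bow attack and an inventory hookup.
; Keyboard axes and a UTC virtual joystick drive movement unless IsAttack is set; Skill1 or Z plays the bow montage.
; BeginPlay spawns UI_Manager and lays out screen-percentage skill and item buttons, of which only Skill1 and Item1 act.
; Item1 adds health potions and refreshes inventory slots; repeated BackKey presses show escalating prompts before quitting.
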(event OnTap(Item1)
  (params (Location :type Vector :default "0, 0, 0") (FingerIndex :type ETouchIndex%20Enum :default "Touch1"))
  (bind _returnvalue (Game|SpawnActorfromClass "/Game/Item/healthPotion.healthPotion_C" (Math|Transform|MakeTransform "0, 0, 0" "0, 0, 0" "1,1,1") "Undefined" 0 0))
  (Class|UIManager|AddItem (Variables|Default|GetUI_Manager) _returnvalue 10)
  (bind _foundwidgets (Widget|GetAllWidgetsOfClass "/Game/UI/InventorySlots.InventorySlots_C" false))
  (for _array_element _foundwidgets
    (Default|UpdateSlot _array_element)))

(event OnYAxisChanged(JoystickComponent)
  (params (Value :type Float%20%28single-precision%29))
  ;[0 1 0] Movement
  (if (not (Variables|Default|GetisAttack))
    (Pawn|Input|AddMovementInput "1.000000,0.000000,0.000000" (* Value 1.0) false)))

(event OnTap(Skill1)
  (params (Location :type Vector :default "0, 0, 0") (FingerIndex :type ETouchIndex%20Enum :default "Touch1"))
  (if (not (Variables|Default|GetisAttack))
    (Variables|Default|SetisAttack true)
    (Animation|Montage|MontagePlay (Components|SkeletalMesh|GetAnimInstance (Variables|Character|GetMesh)) "/Game/Character/Animation/BowAnimMontage.BowAnimMontage" 1.0 "MontageLength" 0.0)))

(event OnXAxisChanged(JoystickComponent)
  (params (Value :type Float%20%28single-precision%29))
  ;[0 1 0] Movement
  (if (not (Variables|Default|GetisAttack))
    (Pawn|Input|AddMovementInput "0.000000,1.000000,0.000000" (* Value 1.0) false)))

(event EventBeginPlay
  (bind _joystickcomponent (Variables|Default|GetJoystickComponent))
  (bind _returnvalue (Game|SpawnActorfromClass "/Script/Amody.UI_Manager" (Math|Transform|MakeTransform "0, 0, 0" "0, 0, 0" "1,1,1") "Undefined" 0 "/Game/UI/MainUI.MainUI_C" "/Game/UI/OnGameUI.OnGameUI_C" 0))
  (Variables|Default|SetUI_Manager _returnvalue)
  (Default|SetupBounds _joystickcomponent true "(X=0.000000,Y=0.600000)" "(X=0.300000,Y=0.400000)" true false)
  (Variables|/Game/JoystickCore/UTCComponent.UTCComponent_C|SetPriority _joystickcomponent 1)
  (Default|SetupWidget _joystickcomponent "/Game/JoystickCore/Widgets/AnimatedWidgets/JoystickWidgetAnimated.JoystickWidgetAnimated_C" true true)
  (CallFunction|SetupSkill)
  (Variables|/Script/Engine.PlayerController|SetbShowMouseCursor (Game|GetPlayerController 0) true))

(event Input|ActionEvents|InputActionBackKey
  (params (Key :type Key%20Structure))
  ;[1 1 1] Exit Game
  (:Pressed
    (switch int (Variables|Default|GetExitTouchCount)
      (:Default
        (Development|ExecuteConsoleCommand "exit" :!label _label))
      (:0
        (Math|Integer|IncrementInt (Variables|Default|GetExitTouchCount)
          (:%20%20
            (Development|PrintString "종료 하시겠습니까?")
            (Utilities|FlowControl|Delay 3.0)
            (Variables|Default|SetExitTouchCount 0))))
      (:1
        (Math|Integer|IncrementInt (Variables|Default|GetExitTouchCount)
          (:%20%20
            (Development|PrintString "진짜 종료 하시겠습니까?"))))
      (:2
        (Math|Integer|IncrementInt (Variables|Default|GetExitTouchCount)
          (:%20%20
            (Development|PrintString "진짜 진짜 종료 하시겠습니까?"))))
      (:3
        (goto _label)))))

(event Input|AxisEvents|InputAxisAxisX
  (params (AxisValue :type Float%20%28single-precision%29))
  ;[0 0 0] Keybord Movemet
  (if (not (Variables|Default|GetisAttack))
    (Pawn|Input|AddMovementInput "1.000000,0.000000,0.000000" (* AxisValue 1.0) false)))

(event Input|AxisEvents|InputAxisAxisY
  (params (AxisValue :type Float%20%28single-precision%29))
  ;[0 0 0] Keybord Movemet
  (if (not (Variables|Default|GetisAttack))
    (Pawn|Input|AddMovementInput "0.000000,1.000000,0.000000" (* 1.0 AxisValue) false)))

(event Input|KeyboardEvents|Z
  (params (Key :type Key%20Structure))
  (:Pressed
    (if (not (Variables|Default|GetisAttack))
      (Variables|Default|SetisAttack true)
      (Animation|Montage|MontagePlay (Components|SkeletalMesh|GetAnimInstance (Variables|Character|GetMesh)) "/Game/Character/Animation/BowAnimMontage.BowAnimMontage" 1.0 "MontageLength" 0.0))))

(event Input|TouchEvents|InputTouch
  (params (Location :type Vector) (FingerIndex :type ETouchIndex%20Enum))
  ;[0 1 0] Movement
  (:Pressed
    (if (not (Variables|Default|GetisUiOpen))
      (Utilities|UTCTouchInputManager Location FingerIndex :!label _label)))
  (:Released
    (goto _label Released))
  (:Moved
    (goto _label Moved)))

(fn ConstructionScript)

(fn SetupSkill
  (bind _skill1 (Variables|Default|GetSkill1))
  (bind _skill2 (Variables|Default|GetSkill2))
  (bind _skill3 (Variables|Default|GetSkill3))
  (bind _skill4 (Variables|Default|GetSkill4))
  (bind _item1 (Variables|Default|GetItem1))
  (bind _item2 (Variables|Default|GetItem2))
  (Utilities|FlowControl|Sequence
    (:then_0
      (Default|SetupBounds _skill1 true "(X=0.900000,Y=0.800000)" "(X=0.000000,Y=0.150000)" true true)
      (Default|SetupBackgroundbyBounds _skill1 "/Game/Skill/BowAttackWidget.BowAttackWidget_C" true)
      (Default|SetupBounds _skill2 true "(X=0.900000,Y=0.600000)" "(X=0.000000,Y=0.150000)" true true)
      (Default|SetupBackgroundbyBounds _skill2 "/Game/Skill/BowAttackWidget.BowAttackWidget_C" true))
    (:then_1
      (Default|SetupBounds _skill3 true "(X=0.900000,Y=0.400000)" "(X=0.000000,Y=0.150000)" true true)
      (Default|SetupBackgroundbyBounds _skill3 "/Game/Skill/BowAttackWidget.BowAttackWidget_C" true)
      (Default|SetupBounds _skill4 true "(X=0.900000,Y=0.200000)" "(X=0.000000,Y=0.150000)" true true)
      (Default|SetupBackgroundbyBounds _skill4 "/Game/Skill/BowAttackWidget.BowAttackWidget_C" true))
    (:then_2
      (Default|SetupBounds _item1 true "(X=0.700000,Y=0.800000)" "(X=0.000000,Y=0.150000)" true true)
      (Default|SetupBackgroundbyBounds _item1 "/Game/Skill/ItemWidget1.ItemWidget1_C" true)
      (Default|SetupBounds _item2 true "(X=0.800000,Y=0.800000)" "(X=0.000000,Y=0.150000)" true true)
      (Default|SetupBackgroundbyBounds _item2 "/Game/Skill/ItemWidget1.ItemWidget1_C" true))))